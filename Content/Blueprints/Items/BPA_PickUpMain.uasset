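; Pickup item actor that takes its mesh and display name, with a count suffix for stacks, from a data table row at construction or through RebuildItem.
; Each tick it turns its name widget toward the player's follow camera and toggles the label's visibility by player distance.
; It also sets the mesh's custom depth stencil to switch the outline highlight when it is the character's ViewedItem.
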(event Custom|Set%20WidgetVisible
  (bind _widgetref (Variables|Default|GetWidgetRef))
  ;[1 1 1] Устанавливает видимость имени предмета
  (Utilities|IsValid _widgetref
    (:Is%20Valid
      (Default|SetVisability _widgetref (Variables|Default|GetWidgetActive)))))

(event Custom|CheckWidget
  ;[1 1 1] Активность надписи
  (if (<= (Math|Vector|Distance(Vector) (Transformation|GetActorLocation (Game|GetPlayerCharacter 0)) (Transformation|GetActorLocation self)) (Variables|Default|GetWidgetVisibleDistance))
    (if (not (Variables|Default|GetWidgetActive))
      (Variables|Default|SetWidgetActive true)
      (CallFunction|SetWidgetVisible))
    (elif (Variables|Default|GetWidgetActive)
      (Variables|Default|SetWidgetActive false)
      (CallFunction|SetWidgetVisible))))

(event Custom|ChangeIteractionColor
  (bind _returnvalue (Game|Player|GetPlayerPawn 0))
  ;[1 1 1] Меняем цвет обводки
  (Utilities|IsValid _returnvalue
    (:Is%20Valid
      (bind _asthird_person_character (Utilities|Casting|CastToThirdPersonCharacter _returnvalue)
        (:then
          (if (== (Variables|/Game/Blueprints/Character/ThirdPersonCharacter.ThirdPersonCharacter_C|GetViewedItem _asthird_person_character) self)
            (if (== (Variables|/Script/Engine.PrimitiveComponent|GetCustomDepthStencilValue (Variables|Debug|GetStaticMeshComponent)) 0)
              (Rendering|SetCustomDepthStencilValue (Variables|Debug|GetStaticMeshComponent) 1))
            (else
              (if true :!label _label
                (Rendering|SetCustomDepthStencilValue (Variables|Debug|GetStaticMeshComponent) 0)))))
        (:CastFailed
          (goto _label))))
    (:Is%20Not%20Valid
      (goto _label))))

(event EventBeginPlay
  ;[1 1 1] Установка имени
  (bind _asbpw_item_name (Utilities|Casting|CastToBPW_ItemName (UserInterface|GetUserWidgetObject (Variables|Default|GetWidget))))
  (Variables|Default|SetWidgetRef _asbpw_item_name)
  (Default|ChangeItemName _asbpw_item_name (Variables|Default|GetItemName))
  (CallFunction|SetWidgetVisible))

(event EventTick
  (params (DeltaSeconds :type Float%20%28single-precision%29))
  ;[1 1 1] Направляем на игрока
  (bind _asthird_person_character (Utilities|Casting|CastToThirdPersonCharacter (Game|GetPlayerCharacter 0)))
  (Transformation|SetWorldRotation (Variables|Default|GetWidget) (Math|Rotator|FindLookatRotation (Transformation|GetWorldLocation (Variables|Default|GetWidget)) (Transformation|GetWorldLocation (Variables|/Script/Weeeel.WeeeelCharacter|GetFollowCamera _asthird_person_character))) false false)
  (CallFunction|ChangeIteractionColor)
  (CallFunction|CheckWidget))

(fn ConstructionScript
  (bind _iteminfo (Variables|Default|GetItemInfo))
  (bind _iteminfo_2 (Variables|Default|GetItemInfo))
  (bind (_datatable _rowname) (Utilities|Struct|BreakDataTableRowHandle (.iteminfo _iteminfo)))
  (bind _returnvalue (Utilities|GetDataTableRow _datatable _rowname)
    (:then
      (Components|StaticMesh|SetStaticMesh (Variables|Debug|GetStaticMeshComponent) (.Mesh (Utilities|Struct|BreakItemData _returnvalue)))
      (if (< (.count _iteminfo_2) 2)
        (Variables|Default|SetItemName (.ItemName (Utilities|Struct|BreakItemData _returnvalue)))
        (else
          (Variables|Default|SetItemName (Utilities|String|StringToName (Utilities|String|Append (Utilities|String|ToString(Name) (.ItemName (Utilities|Struct|BreakItemData _returnvalue))) " x" (Utilities|String|ToString(Integer) (.count _iteminfo_2))))))))))

(fn RebuildItem
  (params (Item :type Item%20Slot%20Structure))
  (bind _widgetref (Variables|Default|GetWidgetRef))
  (Variables|Default|SetItemInfo Item)
  (bind _returnvalue (Utilities|GetDataTableRow (.DataTable (Utilities|Struct|BreakDataTableRowHandle (.iteminfo (Variables|Default|GetItemInfo)))) (.RowName (Utilities|Struct|BreakDataTableRowHandle (.iteminfo (Variables|Default|GetItemInfo)))))
    (:then
      (Components|StaticMesh|SetStaticMesh (Variables|Debug|GetStaticMeshComponent) (.Mesh (Utilities|Struct|BreakItemData _returnvalue)))
      (if (< (.count (Variables|Default|GetItemInfo)) 2)
        (Variables|Default|SetItemName (.ItemName (Utilities|Struct|BreakItemData _returnvalue)))
        (else
          (Variables|Default|SetItemName (Utilities|String|StringToName (Utilities|String|Append (Utilities|String|ToString(Name) (.ItemName (Utilities|Struct|BreakItemData _returnvalue))) " x" (Utilities|String|ToString(Integer) (.count (Variables|Default|GetItemInfo))))))))
      (Utilities|IsValid _widgetref
        (:Is%20Valid
          (Default|ChangeItemName _widgetref (Variables|Default|GetItemName)))
        (:Is%20Not%20Valid
          (Development|PrintString "Ошибка виджета предмета"))))))